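; Placement ghost that previews where a tower will be built.
; Each Tick it traces under the cursor and snaps itself to an XY grid at a fixed height.
; Hitting an existing TowerBP turns the ghost red and clears CanBuild; any other hit turns it green and sets it.
; PlaceTower spawns a TowerBP, passes it TowerData, initializes it and destroys the ghost, without checking CanBuild itself.
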(event `self.ReceiveBeginPlay`)

(event `self.ReceiveTick`
  (params (DeltaSeconds :type "Float (single-precision)"))
  (bind _ghostmesh (`self.GhostMesh`))
  (bind (_hitresult _returnvalue) (`PlayerController.GetHitResultUnderCursorForObjects` (`GameplayStatics.GetPlayerController` 0) (`|MakeArray` "ObjectTypeQuery1" "ObjectTypeQuery3" :!type "EObjectTypeQuery Enum") true))
  (bind _returnvalue_2 (`PrimitiveComponent.GetMaterial` _ghostmesh 0))
  (bind (_bblockinghit _binitialoverlap _time _distance _location _impactpoint _normal _impactnormal _physmat _hitactor) (`GameplayStatics.BreakHitResult` _hitresult))
  (if _returnvalue
    (cast `/Game/Tower/TowerBP` _hitactor
      (:`then`
        (set `self.CanBuild` false)
        (if (not (== _returnvalue_2 "/Game/Tower/RedTranslucent.RedTranslucent"))
          (`PrimitiveComponent.SetMaterial` _ghostmesh 0 "/Game/Tower/RedTranslucent.RedTranslucent")))
      (:`CastFailed`
        (set `self.CanBuild` true)
        (if (not (== _returnvalue_2 "/Game/Tower/GreenTranslucent.GreenTranslucent"))
          (`PrimitiveComponent.SetMaterial` _ghostmesh 0 "/Game/Tower/GreenTranslucent.GreenTranslucent"))))
    (`self.K2_SetActorLocation` (`KismetMathLibrary.MakeVector` (`KismetMathLibrary.GridSnap_Float` (.x _location) 100.0) (`KismetMathLibrary.GridSnap_Float` (.y _location) 100.0) 167.0))))

(event `PlaceTower`
  (bind _returnvalue (`|SpawnActorFromClass` "/Game/Tower/TowerBP.TowerBP_C" (`self.GetTransform`) "AlwaysSpawn" "OverrideRootScale" null null))
  (set `/Game/Tower/TowerBP.TowerStruct` (`self.TowerData`) _returnvalue)
  (`/Game/Tower/TowerBP.TowerInit` _returnvalue)
  (`self.K2_DestroyActor`))

(fn `UserConstructionScript`)