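; Tower actor that automatically fires projectiles at AIRunner enemies entering its range.
; BeginPlay loads a hardcoded test row from the tower data table to set the mesh and detection sphere radius.
; The sphere holds the first entering runner as target until it leaves, without rescanning others already inside.
; Tick spawns projectiles carrying target and damage, throttled by a Reload flag and a FireRate delay.
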(event `self.ReceiveBeginPlay`
  (bind _returnvalue (`|GetDataTableRow` "/Game/Tower/TowerDataTable.TowerDataTable" "TestTower1")
    (:`then`
      (set `self.TowerStruct` _returnvalue)
      (`self.TowerInit`))))

(event `self.ReceiveTick`
  (params (DeltaSeconds :type "Float (single-precision)"))
  (`/Engine/EditorBlueprintResources/StandardMacros.IsValid` (`self.TowerTarget`)
    (:`Is Valid`
      (if (not (`self.Reload`))
        (`self.Shoot`)))))

(event `TowerInit`
  (bind (_name _damage _range _firerate _attacktype _splash _splashrange _splashdamage _shootinglocation _mesh) (break `/Game/Tower/TowerStruct` (`self.TowerStruct`)))
  (`StaticMeshComponent.SetStaticMesh` (`self.Wizard_Tower`) _mesh)
  (`SphereComponent.SetSphereRadius` (`self.Sphere`) _range true))

(event `self.Sphere.OnComponentBeginOverlap`
  (params (OverlappedComponent :type "PrimitiveComponent Object Reference") (OtherActor :type "Actor Object Reference") (OtherComp :type "PrimitiveComponent Object Reference") (OtherBodyIndex :type Integer) (bFromSweep :type Boolean) (SweepResult :type "HitResult Structure (by ref)"))
  (`/Engine/EditorBlueprintResources/StandardMacros.IsValid` (`self.TowerTarget`)
    (:`Is Not Valid`
      (bind _asairunner (cast `/Game/AI/AIRunner` OtherActor))
      (set `self.TowerTarget` _asairunner))))

(event `self.Sphere.OnComponentEndOverlap`
  (params (OverlappedComponent :type "PrimitiveComponent Object Reference") (OtherActor :type "Actor Object Reference") (OtherComp :type "PrimitiveComponent Object Reference") (OtherBodyIndex :type Integer))
  (if (== OtherActor (`self.TowerTarget`))
    (set `self.TowerTarget` null)))

(event `Shoot`
  (bind (_name _damage _range _firerate) (break `/Game/Tower/TowerStruct` (`self.TowerStruct`)))
  (set `self.Reload` true)
  (`|SpawnActorFromClass` "/Game/Tower/TowerProjectile.TowerProjectile_C" (`self.GetTransform`) "AlwaysSpawn" "OverrideRootScale" null (`self.TowerTarget`) _damage null)
  (`KismetSystemLibrary.Delay` _firerate)
  (set `self.Reload` false))

(fn `UserConstructionScript`)